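; BP_EventArgsFactory is a helper that builds and reads typed argument payloads for the global event system.
; Each event type has a Factory function that constructs an EventMessage and appends values, paired with a Parser that reads them back by array index.
; It covers two test events, one carrying an integer and the other a name string plus a position vector.
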(fn `Test2EventArgsFactory`
  (params (Name :type String) (Postion :type "Vector Structure"))
  (returns (Message :type "/Game/GlobalEventSystem/EventMessage Object Reference"))
  (bind _returnvalue (`|GenericCreateObject` "/Game/GlobalEventSystem/EventMessage.EventMessage_C"))
  (`/Game/GlobalEventSystem/EventMessage.AddString` _returnvalue Name)
  (`/Game/GlobalEventSystem/EventMessage.AddVector` _returnvalue Postion)
  (return _returnvalue))

(fn `Test2EventArgsParser`
  (params (Message :type "/Game/GlobalEventSystem/EventMessage Object Reference"))
  (returns (Name :type String) (Position :type "Vector Structure"))
  (bind _args (`/Game/GlobalEventSystem/EventMessage.Args` Message))
  (return (`/Game/GlobalEventSystem/ExtendedVariable.StringValue` (`|GetArrayItem` _args)) (`/Game/GlobalEventSystem/ExtendedVariable.VectorValue` (`|GetArrayItem` _args 1))))

(fn `TestEventArgsFactory`
  (params (TestIntValue :type Integer))
  (returns (Message :type "/Game/GlobalEventSystem/EventMessage Object Reference"))
  (bind _returnvalue (`|GenericCreateObject` "/Game/GlobalEventSystem/EventMessage.EventMessage_C"))
  (`/Game/GlobalEventSystem/EventMessage.AddInt` _returnvalue TestIntValue)
  (return _returnvalue))

(fn `TestEventArgsParser`
  (params (Message :type "/Game/GlobalEventSystem/EventMessage Object Reference"))
  (returns (IntValue :type Integer))
  (return (`/Game/GlobalEventSystem/ExtendedVariable.IntValue` (`|GetArrayItem` (`/Game/GlobalEventSystem/EventMessage.Args` Message)))))