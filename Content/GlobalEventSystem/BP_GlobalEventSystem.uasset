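; Global event bus Blueprint that relays typed events, such as player death, to registered subscribers.
; Init builds an array with one subscriber-list struct per E_EventType value, indexed by the enum's integer, and AddSubscriber appends to the matching list.
; CastEvent switches on the type and passes the message to each subscriber through that type's dedicated callback, so each event type has its own hand-wired branch.
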(event `Init`
  (foreach `/Game/GlobalEventSystem/E_EventType` false
    (:`LoopBody`
      (`KismetArrayLibrary.Array_Add` (`self.Events`) (make `/Game/GlobalEventSystem/S_SubscribersList` _)))))

(event `AddSubscriber`
  (params (EventType :type "/Game/GlobalEventSystem/E_EventType Enum" :default "NewEnumerator0") (Subscriber :type "/Game/GlobalEventSystem/I_Subscriber Interface"))
  (`KismetArrayLibrary.Array_Add` (`.MemberVar_0_2_7C3E6D2442E1577C0EC4CFB7BE9B20A4` (break `/Game/GlobalEventSystem/S_SubscribersList` (`|GetArrayItem` (`self.Events`) (`KismetMathLibrary.Conv_ByteToInt` EventType)))) Subscriber))

(event `CastEvent`
  (params (EventType :type "/Game/GlobalEventSystem/E_EventType Enum" :default "NewEnumerator0") (Message :type "/Game/GlobalEventSystem/EventMessage Object Reference"))
  (bind _returnvalue (`KismetMathLibrary.Conv_ByteToInt` EventType))
  (switch `/Game/GlobalEventSystem/E_EventType` EventType
    (:`NewEnumerator4`
      (for _array_element (`.MemberVar_0_2_7C3E6D2442E1577C0EC4CFB7BE9B20A4` (break `/Game/GlobalEventSystem/S_SubscribersList` (`|GetArrayItem` (`self.Events`) _returnvalue)))
        (`/Game/GlobalEventSystem/I_Subscriber.TestFuncCallbabk` _array_element Message)))
    (:`NewEnumerator3`
      (for _array_element_2 (`.MemberVar_0_2_7C3E6D2442E1577C0EC4CFB7BE9B20A4` (break `/Game/GlobalEventSystem/S_SubscribersList` (`|GetArrayItem` (`self.Events`) _returnvalue)))
        (`/Game/GlobalEventSystem/I_Subscriber.PlayerDeathCallback` _array_element_2 Message)))
    (:`NewEnumerator5`
      (for _array_element_3 (`.MemberVar_0_2_7C3E6D2442E1577C0EC4CFB7BE9B20A4` (break `/Game/GlobalEventSystem/S_SubscribersList` (`|GetArrayItem` (`self.Events`) _returnvalue)))
        (`/Game/GlobalEventSystem/I_Subscriber.TestFunc2Callback` _array_element_3 Message)))))